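; Game manager for a card game that builds two players' decks from their Tokou characters and draws from the first.
; The Test event fills both deck arrays with fixed repeats of each Tokou's seven cards.
; DrawCard stores a random pick from the returned first deck as ActualCard, prints a debug string, then calls Remove on Deck1Array, which strips every copy of that card.
; Deck 2 is built but never drawn.
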(event `self.ReceiveBeginPlay`)

(event `Test`
  (params (`Tokou 1` :type "/Game/Blueprints/BP_Tokou Object Reference") (`Tokou 2` :type "/Game/Blueprints/BP_Tokou Object Reference"))
  (bind _deck_1 (`self.CreateDeckFromTokouCards` `Tokou 1` `Tokou 2`)))

(event `DrawCard`
  (`self.DrawRandomCard` (stale `Test` _deck_1)))

(fn `CreateDeckFromTokouCards`
  (params (`Tokou 1` :type "/Game/Blueprints/BP_Tokou Object Reference") (`Tokou 2` :type "/Game/Blueprints/BP_Tokou Object Reference"))
  (returns (`Deck 1` :type "Array of /Game/Blueprints/BP_Card Object Reference") (`Deck 2` :type "Array of /Game/Blueprints/BP_Card Object Reference"))
  (bind _card1ac (`/Game/Blueprints/BP_Tokou.Card1AC` `Tokou 1`))
  (bind _card2ac (`/Game/Blueprints/BP_Tokou.Card2AC` `Tokou 1`))
  (bind _card3ad (`/Game/Blueprints/BP_Tokou.Card3AD` `Tokou 1`))
  (bind _card4ad (`/Game/Blueprints/BP_Tokou.Card4AD` `Tokou 1`))
  (bind _card5spe (`/Game/Blueprints/BP_Tokou.Card5SPE` `Tokou 1`))
  (bind _card6spe (`/Game/Blueprints/BP_Tokou.Card6SPE` `Tokou 1`))
  (bind _card7sa (`/Game/Blueprints/BP_Tokou.Card7SA` `Tokou 1`))
  (bind _card1ac_2 (`/Game/Blueprints/BP_Tokou.Card1AC` `Tokou 2`))
  (bind _card2ac_2 (`/Game/Blueprints/BP_Tokou.Card2AC` `Tokou 2`))
  (bind _card3ad_2 (`/Game/Blueprints/BP_Tokou.Card3AD` `Tokou 2`))
  (bind _card4ad_2 (`/Game/Blueprints/BP_Tokou.Card4AD` `Tokou 2`))
  (bind _card5spe_2 (`/Game/Blueprints/BP_Tokou.Card5SPE` `Tokou 2`))
  (bind _card6spe_2 (`/Game/Blueprints/BP_Tokou.Card6SPE` `Tokou 2`))
  (bind _card7sa_2 (`/Game/Blueprints/BP_Tokou.Card7SA` `Tokou 2`))
  (`KismetArrayLibrary.Array_Clear` (`self.Deck1Array`))
  (`KismetArrayLibrary.Array_Clear` (`self.Deck2Array`))
  (bind _output_get (set `self.Deck1Array` (`|MakeArray` _card1ac _card1ac _card1ac _card1ac _card1ac _card2ac _card2ac _card2ac _card2ac _card2ac _card3ad _card3ad _card3ad _card3ad _card3ad _card4ad _card4ad _card4ad _card4ad _card4ad _card5spe _card5spe _card5spe _card5spe _card5spe _card6spe _card6spe _card6spe _card6spe _card6spe _card7sa _card7sa _card7sa)))
  (bind _output_get_2 (set `self.Deck2Array` (`|MakeArray` _card1ac_2 _card1ac_2 _card1ac_2 _card1ac_2 _card1ac_2 _card2ac_2 _card2ac_2 _card2ac_2 _card2ac_2 _card2ac_2 _card3ad_2 _card3ad_2 _card3ad_2 _card3ad_2 _card3ad_2 _card4ad_2 _card4ad_2 _card4ad_2 _card4ad_2 _card4ad_2 _card5spe_2 _card5spe_2 _card5spe_2 _card5spe_2 _card5spe_2 _card6spe_2 _card6spe_2 _card6spe_2 _card6spe_2 _card6spe_2 _card7sa_2 _card7sa_2 _card7sa_2)))
  (return _output_get _output_get_2))

(fn `DrawRandomCard`
  (params (`Deck 1` :type "Array of /Game/Blueprints/BP_Card Object Reference"))
  (bind _output_get (set `self.ActualCard` (`KismetArrayLibrary.Array_Random` `Deck 1`)))
  (`KismetSystemLibrary.PrintString` "Hello")
  (`KismetArrayLibrary.Array_RemoveItem` (`self.Deck1Array`) _output_get)
  (return))

(fn `UserConstructionScript`)